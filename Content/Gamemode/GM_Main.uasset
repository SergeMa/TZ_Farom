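; GM_Main is the game mode for a two-player ball game, handling player spawn assignment and match start.
; Tick polls the player count, printing a waiting message unless exactly two are present, then spawns BP_Ball once at a fixed location, guarded by GameStarted.
; A ChoosePlayerStart override returns the first unclaimed PlayerStart and retags it "PlayerSpawned" so each player gets a separate start.
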(event EventBeginPlay)

(event EventTick
  (params (DeltaSeconds :type Float%20%28single-precision%29))
  (bind _returnvalue (Class|GameModeBase|GetNumPlayers))
  (if (== _returnvalue 2)
    (if (not (Variables|Default|GetGameStarted))
      (Game|SpawnActorfromClass "/Game/Blueprints/BP_Ball.BP_Ball_C" (Math|Transform|MakeTransform "540.000000,1500.000000,170.000000" "0, 0, 0" "1,1,1") "Undefined" 0 0)
      (Variables|Default|SetGameStarted true))
    (else
      (Development|PrintString "Not all players connected"))))

(fn ConstructionScript)

(fn ChoosePlayerStart
  (params (Player :type Controller%20Object%20Reference))
  (bind _outactors (Actor|GetAllActorsOfClass "/Script/Engine.PlayerStart"))
  (for _array_element _outactors
    (if (Utilities|Name|NotEqual(Name) (Variables|/Script/Engine.PlayerStart|GetPlayerStartTag _array_element) "PlayerSpawned")
      (Variables|/Script/Engine.PlayerStart|SetPlayerStartTag _array_element "PlayerSpawned")
      (return _array_element))))